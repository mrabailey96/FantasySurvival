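; BP_DamageNumberActor is a short-lived actor that shows a floating damage number.
; On BeginPlay it passes Amount to the WBP_DamageNumber widget in its WCDamage component and sets its lifespan from Lifetime.
; Each tick it moves upward in world space at RiseSpeed, scaled by delta time.
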(event EventBeginPlay
  (bind _aswbp_damage_number (Utilities|Casting|CastToWBP_DamageNumber (UserInterface|GetUserWidgetObject (Variables|Default|GetWC_Damage))))
  (Default|Init _aswbp_damage_number (Variables|Default|GetAmount))
  (Actor|SetLifeSpan (Variables|Default|GetLifetime)))

(event EventTick
  (params (DeltaSeconds :type Float%20%28single-precision%29))
  (Transformation|AddActorWorldOffset (Math|Vector|MakeVector 0.0 0.0 (* (Variables|Default|GetRiseSpeed) DeltaSeconds))))

(fn ConstructionScript)